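; Main player character that executes a programmed sequence of action cards: moves, turns and elemental effects.
; PlaySequence dispatches each card to BPMoveForward or BPEffects, and NextAction advances the index after each timeline finishes or effect is triggered.
; Card removal records indices for later adds, which write MoveForward at the lowest one instead of the passed card.
; It also creates the HUD and prints its transform every tick for debugging.
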(event `self.ReceiveTick`
  (params (DeltaSeconds :type "Float (single-precision)"))
  ;[1 0 0] Tick / DEBUG
  (`KismetSystemLibrary.PrintString` (`KismetStringLibrary.Concat_StrStr` "Player Location : " (`KismetStringLibrary.Conv_VectorToString` (`self.K2_GetActorLocation`)) " | Player Rotation : " (`KismetStringLibrary.Conv_RotatorToString` (`self.K2_GetActorRotation`))) true true (struct :`G` 0.66 :`B` 1.0 :`A` 1.0) 0.0))

(event `self.ReceiveBeginPlay`
  (bind _returnvalue (`|CreateWidget` "/Game/Blueprint/UI/WBP_HUD.WBP_HUD_C"))
  (`UserWidget.AddToViewport` _returnvalue 0)
  (set `/Game/Blueprint/BP_MoveForward.PlayerRef` self (`self.BP_MoveForward`))
  (set `/Game/Blueprint/Effects/BP_Effects.Owner` self (`self.BP_Effects`)))

(event `Play Effect`
  (params (Effect :type "/Game/Blueprint/Effects/Enum_Effects Enum" :default "NewEnumerator0"))
  ;[0.2667 1 0.702] Activate Element
  (`/Game/Blueprint/Effects/BP_Effects.PlayEffect` (`self.BP_Effects`) Effect)
  (`self.NextAction`))

(event `MoveToDestination`
  (params (LastDestination :type "Vector Structure"))
  ;[0.3412 1 0.2549] Movement
  (bind (_direction _movetolocation) (`Timeline|Timeline` :!via `PlayFromStart`)
    (:`Update`
      (`self.K2_SetActorLocation` (`KismetMathLibrary.VLerp` (`self.K2_GetActorLocation`) LastDestination _movetolocation)))
    (:`Finished`
      (`self.NextAction`))))

(event `Set Current Effect`
  (params (`current effect` :type "/Game/Blueprint/Effects/Enum_Effects Enum" :default "NewEnumerator0"))
  ;[0.1373 0.1373 0.1373 0.6667] Change Element (Obsolete)
  (set `self.current effect` `current effect`))

(event `RotationLeft`
  (params (NewRotation :type "Rotator Structure"))
  ;[0.3405 1 0.2532] Rotation (Left)
  (bind (_direction _rotaleft) (`Timeline|Timeline_0` :!via `PlayFromStart`)
    (:`Update`
      (`self.K2_SetActorRotation` (`KismetMathLibrary.RLerp` (`self.K2_GetActorRotation`) NewRotation _rotaleft true)))
    (:`Finished`
      (`self.NextAction`))))

(event `RotationRight`
  (params (NewRotation :type "Rotator Structure"))
  ;[0.3412 1 0.2549] Rotation (Right)
  (bind (_direction _leftrota) (`Timeline|Timeline_1` :!via `PlayFromStart`)
    (:`Update`
      (`self.K2_SetActorRotation` (`KismetMathLibrary.RLerp` (`self.K2_GetActorRotation`) NewRotation _leftrota true)))
    (:`Finished`
      (`self.NextAction`))))

(event `NextAction`
  ;[0.3412 1 0.2549] Go To Next Action
  (bind _result (`/Engine/EditorBlueprintResources/StandardMacros.IncrementInt` (`self.IndexSequence`))
    (:`  `
      (if (not (> _result (`KismetArrayLibrary.Array_LastIndex` (`self.E_Action`))))
        (`self.Play Sequence`)))))

(event `RemoveCardInSequence`
  (params (IndexToRemove :type Integer))
  ;[0.4039 0.3373 1] Remove Card in Sequence
  (`KismetArrayLibrary.Array_Remove` (`self.E_Action`) IndexToRemove)
  (set `self.CardHasBeenRemoved` true)
  (`KismetArrayLibrary.Array_Add` (`self.HolesInSequence`) IndexToRemove))

(event `Play Sequence`
  (bind _bp_moveforward (`self.BP_MoveForward`))
  ;[0.4039 0.3373 1] Play Sequence
  (switch `/Game/Blueprint/E_ActionPlayer` (`|GetArrayItem` (`self.E_Action`) (`self.IndexSequence`))
    (:`NewEnumerator0`
      (`/Game/Blueprint/BP_MoveForward.MoveForward` _bp_moveforward))
    (:`NewEnumerator1`
      (`/Game/Blueprint/BP_MoveForward.TurnLeft` _bp_moveforward))
    (:`NewEnumerator2`
      (`/Game/Blueprint/BP_MoveForward.TurnRight` _bp_moveforward))
    (:`NewEnumerator3`
      (`self.Set Current Effect` "NewEnumerator1")
      (`self.Play Effect` (`self.current effect`) :!label _label))
    (:`NewEnumerator4`
      (`self.Set Current Effect` "NewEnumerator0")
      (goto _label))
    (:`NewEnumerator5`
      (`self.Set Current Effect` "NewEnumerator2")
      (goto _label))
    (:`NewEnumerator6`
      (`self.Set Current Effect` "NewEnumerator3")
      (goto _label))))

(event `AddCardInSequence`
  (params (`New Card` :type "/Game/Blueprint/E_ActionPlayer Enum (by ref)"))
  (bind _e_action (`self.E_Action`))
  ;[0.4025 0.3379 1] Add Card in Sequence
  (if (`self.CardHasBeenRemoved`)
    (`self.Smallest Card`)
    (`KismetArrayLibrary.Array_Set` _e_action (`self.CurrentSmallest`) "NewEnumerator0")
    (else
      (`KismetArrayLibrary.Array_Add` _e_action `New Card`))))

(event `Smallest Card`
  (bind _holesinsequence (`self.HolesInSequence`))
  ;[0.4039 0.3373 1] Find Smallest Removed Card
  (if (== (`KismetArrayLibrary.Array_Length` _holesinsequence) 1)
    (set `self.CurrentSmallest` (`|GetArrayItem` _holesinsequence))
    (set `self.CardHasBeenRemoved` false)
    (else
      (set `self.CurrentSmallest` (`|GetArrayItem` _holesinsequence))
      (for _array_element _holesinsequence
        (if (< _array_element (`self.CurrentSmallest`))
          (set `self.CurrentSmallest` _array_element))))))

(event `GetKilled`)

(fn `UserConstructionScript`)