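; BP_Effects plays the player's elemental effects (Fire, Water, Earth or Wind) and applies them to nearby traps.
; PlayEffect switches on the element to spawn its Niagara system at the owner's location and orientation, with a matching 2D sound.
; It then calls DisableTrap with that element on every ProtoTrap overlapping the owner's EffectCollision.
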(event `PlayEffect`
  (params (Effect :type "/Game/Blueprint/Player/Effects/Enum_Effects Enum" :default "NewEnumerator0"))
  (bind (_location _rotation) (`self.Niagara Loc&Rot`))
  (bind (_location_2 _rotation_2) (`self.Niagara Loc&Rot`))
  (switch `/Game/Blueprint/Player/Effects/Enum_Effects` Effect
    (:`NewEnumerator0`
      (`NiagaraFunctionLibrary.SpawnSystemAtLocation` "/Game/Blueprint/SFX/NS_TemporaryFlames.NS_TemporaryFlames" _location _rotation)
      (`GameplayStatics.PlaySound2D` "/Game/SoundDesign/SC/FireActivation_Cue.FireActivation_Cue" 1.0 1.0 0.0 null null))
    (:`NewEnumerator1`
      (`NiagaraFunctionLibrary.SpawnSystemAtLocation` "/Game/Blueprint/SFX/NS_TemporaryWater.NS_TemporaryWater" _location _rotation)
      (`GameplayStatics.PlaySound2D` "/Game/SoundDesign/SC/SC_Water.SC_Water" 1.0 1.0 0.0 null null))
    (:`NewEnumerator2`
      (`NiagaraFunctionLibrary.SpawnSystemAtLocation` "/Game/Blueprint/SFX/NS_TemporaryEarth.NS_TemporaryEarth" _location_2 _rotation_2)
      (`GameplayStatics.PlaySound2D` "/Game/SoundDesign/SoundWave/EarthUse.EarthUse" 1.0 1.0 0.0 null null))
    (:`NewEnumerator3`
      (`NiagaraFunctionLibrary.SpawnSystemAtLocation` "/Game/Blueprint/SFX/NS_TemporaryWind.NS_TemporaryWind" _location_2 _rotation_2)
      (`GameplayStatics.PlaySound2D` "/Game/SoundDesign/SoundWave/Wind.Wind" 1.0 1.0 0.0 null null)))
  (for _array_element (`PrimitiveComponent.GetOverlappingActors` (`/Game/Blueprint/Player/BP_MainCharacter.Effect Collision` (`self.Owner`)) null)
    (bind _asproto_trap (cast `/Game/Blueprint/Player/Effects/ProtoTraps/ProtoTrap` _array_element))
    (`/Game/Blueprint/Player/Effects/ProtoTraps/ProtoTrap.Disable trap` _asproto_trap Effect)))

(fn `Niagara Loc&Rot`
  (returns (Location :type "Vector Structure") (Rotation :type "Rotator Structure"))
  (bind _owner (`self.Owner`))
  (return (`Actor.K2_GetActorLocation` _owner) (`KismetMathLibrary.MakeRotationFromAxes` (`Actor.GetActorForwardVector` _owner) (`Actor.GetActorRightVector` _owner) (`Actor.GetActorUpVector` _owner))))