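; Test character for trying out player effects, driven by hard-coded debug keys.
; Space plays the current effect through BPEffects, and R cycles the selection through three effect types.
; Z teleport-steps the character forward unless EffectArea overlaps a ProtoTrap, while E makes a wind-boosted step of double length with no trap check.
; BeginPlay sets the BPEffects owner to None rather than to this character.
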(event `self.ReceiveBeginPlay`
  (set `/Game/Blueprint/Player/Effects/BP_Effects.Owner` null (`self.BP_Effects`)))

(event `Key|SpaceBar`
  (params (Key :type "Key Structure"))
  ;[1 1 1] Effects
  (:`Pressed`
    (`/Game/Blueprint/Player/Effects/BP_Effects.PlayEffect` (`self.BP_Effects`) (`self.current effect`))))

(event `Key|R`
  (params (Key :type "Key Structure"))
  ;[1 1 1] Effects
  (:`Pressed`
    (set `self.current effect` (cast `/Game/Blueprint/Player/Effects/Enum_Effects` (mod (+ (`self.current effect`) 1) 3)))))

(event `Key|Z`
  (params (Key :type "Key Structure"))
  ;[1 1 1] Fuck you "insert debug movement"
  (:`Pressed`
    (for _array_element (`PrimitiveComponent.GetOverlappingActors` (`self.EffectArea`) null)
      (cast `/Game/Blueprint/Player/Effects/ProtoTraps/ProtoTrap` _array_element)
      (bind _output_get (set `self.GotObstacle` true)))
    (if _output_get
      (set `self.GotObstacle` false)
      (else
        (`self.GoForward` false)))))

(event `GoForward`
  (params (`WindBoosted?` :type Boolean))
  ;[1 1 1] Fuck you "insert debug movement"
  (`self.K2_SetActorLocation` (+ (* (* (+ `WindBoosted?` 1) 100.0) (`self.GetActorForwardVector`)) (`self.K2_GetActorLocation`))))

(event `Key|E`
  (params (Key :type "Key Structure"))
  ;[1 1 1] Fuck you "insert debug movement"
  (:`Pressed`
    (`self.GoForward` true)))

(fn `UserConstructionScript`)