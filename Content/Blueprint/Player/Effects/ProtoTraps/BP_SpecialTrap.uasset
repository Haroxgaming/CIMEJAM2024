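; BP_SpecialTrap is a trigger that spawns a proto trap when the main character walks into it.
; It caches the player on BeginPlay and reacts to box overlaps from that player, ignoring the player's EffectCollision component.
; On the first valid overlap it spawns a ProtoTrap at TrapSpawn's transform, passing it the trap type and itself, then latches so it fires only once.
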(event `self.ReceiveBeginPlay`
  (bind _returnvalue (`GameplayStatics.GetActorOfClass` "/Game/Blueprint/Player/BP_MainCharacter.BP_MainCharacter_C"))
  (set `self.Player ref` _returnvalue))

(event `self.Box.OnComponentBeginOverlap`
  (params (OverlappedComponent :type "PrimitiveComponent Object Reference") (OtherActor :type "Actor Object Reference") (OtherComp :type "PrimitiveComponent Object Reference") (OtherBodyIndex :type Integer) (bFromSweep :type Boolean) (SweepResult :type "HitResult Structure (by ref)"))
  (bind _player_ref (`self.Player ref`))
  (if (not (`self.Spawned`))
    (if (and (== OtherActor _player_ref) (not (== OtherComp (`/Game/Blueprint/Player/BP_MainCharacter.Effect Collision` _player_ref))))
      (bind _returnvalue (`|SpawnActorFromClass` "/Game/Blueprint/Player/Effects/ProtoTraps/ProtoTrap.ProtoTrap_C" (`SceneComponent.K2_GetComponentToWorld` (`self.TrapSpawn`)) "Undefined" "MultiplyWithRoot" null (`self.TrapToSpawn`) self null))
      (set `self.TrapSpawned` _returnvalue)
      (set `self.Spawned` true))))

(fn `UserConstructionScript`)