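; Player character that executes a queued sequence of action cards: moves, turns, diagonals and water, fire, earth or air effects.
; PlaySequence switches on the current action and delegates to BPMoveForward or BPEffects, with a forward trace triggering a bump when blocked.
; Timelines lerp location and rotation, calling NextAction on finish to advance the queue.
; Also handles card add/remove, checkpoint HUD updates, and respawning at the checkpoint with its traps re-enabled.
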(event `self.ReceiveTick`
  (params (DeltaSeconds :type "Float (single-precision)"))
  ;[1 0 0] Tick / DEBUG
  (`KismetSystemLibrary.PrintString` (`KismetStringLibrary.Conv_IntToString` (`self.IndexSequence`)) true true (struct :`R` 0.78073 :`G` 1.0 :`A` 1.0) 0.0))

(event `self.ReceiveBeginPlay`
  ;[1 0.1216 0.5569] Begin play
  (bind _returnvalue (`|CreateWidget` "/Game/Blueprint/UI/WBP_HUD.WBP_HUD_C"))
  (set `self.HUD ref` _returnvalue)
  (`UserWidget.AddToViewport` _returnvalue 0)
  (set `/Game/Blueprint/Player/MoveForward/BP_MoveForward.PlayerRef` self (`self.BP_MoveForward`))
  (set `/Game/Blueprint/Player/Effects/BP_Effects.Owner` self (`self.BP_Effects`))
  (`KismetMaterialLibrary.CreateDynamicMaterialInstance` "/Game/Gameart/Esteban/MI_air.MI_air"))

(event `Play Effect`
  (params (Effect :type "/Game/Blueprint/Player/Effects/Enum_Effects Enum" :default "NewEnumerator0"))
  ;[0.2667 1 0.702] Activate Element
  (`/Game/Blueprint/Player/Effects/BP_Effects.PlayEffect` (`self.BP_Effects`) Effect)
  (`KismetSystemLibrary.Delay` 1.0)
  (`self.NextAction`))

(event `MoveToDestination`
  (params (LastDestination :type "Vector Structure"))
  ;[0.3412 1 0.2549] Movement
  (bind (_direction _movetolocation) (`Timeline|Timeline` :!via `PlayFromStart` :!label _label)
    (:`Update`
      (`self.K2_SetActorLocation` (`KismetMathLibrary.VLerp` (`self.K2_GetActorLocation`) LastDestination _movetolocation)))
    (:`Finished`
      (`self.NextAction`))))

(event `CantMove`
  (bind _jumpstart (`self.JumpStart`))
  ;[0.3412 1 0.2549] Get Bonked!
  (set `self.JumpStart` (`self.K2_GetActorLocation`))
  (bind (_direction _newtrack_0) (`Timeline|Timeline_4` :!via `PlayFromStart` :!label _label_2)
    (:`Update`
      (`self.K2_SetActorLocation` (`KismetMathLibrary.VLerp` _jumpstart (+ _jumpstart (`self.Jump`)) _newtrack_0)))
    (:`Finished`
      (`self.NextAction`))))

(event `Set Current Effect`
  (params (`current effect` :type "/Game/Blueprint/Player/Effects/Enum_Effects Enum" :default "NewEnumerator0"))
  ;[0.2667 1 0.702] Change Element
  (set `self.current effect` `current effect`))

(event `Checkpoint`
  (params (MaxBuy :type Integer))
  (bind _hud_ref (`self.HUD ref`))
  ;[0.1059 0.05882 0.5137] Reached Checkpoint
  (`KismetSystemLibrary.Delay` 0.5)
  (bind _output_get (set `/Game/Blueprint/UI/WBP_HUD.MaxBuy` MaxBuy _hud_ref))
  (`/Game/Blueprint/UI/WBP_HUD.Zone change` _hud_ref _output_get)
  (`GameplayStatics.PlaySound2D` "/Game/SoundDesign/SC/CheckPoint_Cue.CheckPoint_Cue" 1.0 1.0 0.0 null null))

(event `Stop Timelines`
  ;[1 1 1] Stop Moving
  (`|ExecutionSequence`
    (:`then_0`
      (goto _label_2 :!via `Stop`))
    (:`then_1`
      (goto _label :!via `Stop`))
    (:`then_2`
      ;[0.3412 1 0.2549] Diagonal Bas
      (bind (_direction _movetolocation) (`Timeline|Timeline_3` :!via `Stop` :!label _label_3)
        (:`Update`
          (`self.K2_SetActorLocation` (`KismetMathLibrary.VLerp` (`self.K2_GetActorLocation`) (stale `DiagonalDown` InputPin) _movetolocation)))
        (:`Finished`
          (`self.NextAction`))))
    (:`then_3`
      ;[0.3405 1 0.2532] Rotation (Left)
      (bind (_direction_2 _rotaleft) (`Timeline|Timeline_0` :!via `Stop` :!label _label_4)
        (:`Update`
          (`self.K2_SetActorRotation` (`KismetMathLibrary.RLerp` (`self.K2_GetActorRotation`) (stale `RotationLeft` NewRotation) _rotaleft true)))
        (:`Finished`
          (`self.NextAction`))))
    (:`then_4`
      ;[0.3412 1 0.2549] Rotation (Right)
      (bind (_direction_3 _leftrota) (`Timeline|Timeline_1` :!via `Stop` :!label _label_5)
        (:`Update`
          (`self.K2_SetActorRotation` (`KismetMathLibrary.RLerp` (`self.K2_GetActorRotation`) (stale `RotationRight` NewRotation) _leftrota true)))
        (:`Finished`
          (`self.NextAction`))))
    (:`then_5`
      ;[0.3412 1 0.2549] Diagonal Up
      (bind (_direction_4 _movetolocation_2) (`Timeline|Timeline_2` :!via `Stop` :!label _label_6)
        (:`Update`
          (`self.K2_SetActorLocation` (`KismetMathLibrary.VLerp` (`self.K2_GetActorLocation`) (stale `Diagonal Up` InputPin) _movetolocation_2)))
        (:`Finished`
          (`self.NextAction`))))))

(event `DiagonalDown`
  (params (InputPin :type "Vector Structure"))
  ;[0.3412 1 0.2549] Diagonal Bas
  (goto _label_3 :!via `PlayFromStart`))

(event `RotationLeft`
  (params (NewRotation :type "Rotator Structure"))
  ;[0.3405 1 0.2532] Rotation (Left)
  (goto _label_4 :!via `PlayFromStart`))

(event `Change PlayRate`
  (params (NewRate :type "Float (single-precision)"))
  ;[0.3412 1 0.2549] Switch PlayRate
  (`TimelineComponent.SetPlayRate` (`self.Timeline_1`) NewRate)
  (`TimelineComponent.SetPlayRate` (`self.Timeline_0`) NewRate)
  (`TimelineComponent.SetPlayRate` (`self.Timeline`) NewRate)
  (`TimelineComponent.SetPlayRate` (`self.Timeline_2`) NewRate)
  (`TimelineComponent.SetPlayRate` (`self.Timeline_3`) NewRate))

(event `Diagonal Up`
  (params (InputPin :type "Vector Structure"))
  ;[0.3412 1 0.2549] Diagonal Up
  (goto _label_6 :!via `PlayFromStart`))

(event `RotationRight`
  (params (NewRotation :type "Rotator Structure"))
  ;[0.3412 1 0.2549] Rotation (Right)
  (goto _label_5 :!via `PlayFromStart`))

(event `NextAction`
  ;[0.3412 1 0.2549] Go To Next Action
  (bind _result (`/Engine/EditorBlueprintResources/StandardMacros.IncrementInt` (`self.IndexSequence`))
    (:`  `
      (if (not (> _result (`KismetArrayLibrary.Array_LastIndex` (`self.E_Action`))))
        (`self.Play Sequence`)
        (else
          (set `self.SequenceIsOver` true))))))

(event `RemoveCardInSequence`
  (params (IndexToRemove :type Integer))
  ;[0.4039 0.3373 1] Remove Card in Sequence
  (`KismetArrayLibrary.Array_Remove` (`self.E_Action`) IndexToRemove)
  (set `self.ReadyToAdd` true)
  (`KismetArrayLibrary.Array_Add` (`self.HolesInSequence`) IndexToRemove))

(event `Play Sequence`
  (bind _returnvalue (`self.K2_GetActorLocation`))
  (bind _bp_moveforward (`self.BP_MoveForward`))
  (bind _bp_moveforward_2 (`self.BP_MoveForward`))
  (bind _output (`|GetArrayItem` (`self.E_Action`) (`self.IndexSequence`)))
  ;[0.4039 0.3373 1] Play Sequence
  (`KismetSystemLibrary.PrintString` (`KismetStringLibrary.Conv_IntToString` (`self.IndexSequence`)))
  (set `self.SequenceIsOver` false)
  (if (`self.Something in sequence`)
    (`KismetSystemLibrary.PrintString` (`|GetEnumeratorNameAsString` _output) true true (struct :`G` 0.66 :`B` 1.0 :`A` 1.0) 5.0)
    (switch `/Game/Blueprint/Player/MoveForward/E_ActionPlayer` _output
      (:`NewEnumerator0`
        (bind (_outhit _returnvalue_2) (`KismetSystemLibrary.LineTraceSingle` _returnvalue (+ _returnvalue (* 100.0 (`self.GetActorForwardVector`))) "TraceTypeQuery1"))
        (if (or (not _returnvalue_2) (`self.Cinematic`))
          (`/Game/Blueprint/Player/MoveForward/BP_MoveForward.MoveForward` _bp_moveforward_2)
          (else
            (`self.CantMove`)))
        (if (== (+ (`self.IndexSequence`) 1) (`KismetArrayLibrary.Array_Length` (`self.E_Action`))) :!label _label_7
          (set `self.Something in sequence` false)
          (`KismetSystemLibrary.Delay` 3.0)
          (if (`self.CanRespawn`)
            (`self.GetRespawned`))))
      (:`NewEnumerator1`
        (`/Game/Blueprint/Player/MoveForward/BP_MoveForward.TurnLeft` _bp_moveforward_2)
        (goto _label_7))
      (:`NewEnumerator2`
        (`/Game/Blueprint/Player/MoveForward/BP_MoveForward.TurnRight` _bp_moveforward_2)
        (goto _label_7))
      (:`NewEnumerator3`
        (`self.Set Current Effect` "NewEnumerator1")
        (`self.Play Effect` (`self.current effect`) :!label _label_8)
        (goto _label_7))
      (:`NewEnumerator4`
        (`self.Set Current Effect` "NewEnumerator0")
        (goto _label_8))
      (:`NewEnumerator5`
        (`self.Set Current Effect` "NewEnumerator2")
        (goto _label_8))
      (:`NewEnumerator6`
        (`self.Set Current Effect` "NewEnumerator3")
        (goto _label_8))
      (:`NewEnumerator7`
        (`/Game/Blueprint/Player/MoveForward/BP_MoveForward.DiagonalUp` _bp_moveforward))
      (:`NewEnumerator8`
        (`/Game/Blueprint/Player/MoveForward/BP_MoveForward.DiagonalDown` _bp_moveforward)))))

(event `AddCardInSequence`
  (params (`New Card` :type "/Game/Blueprint/Player/MoveForward/E_ActionPlayer Enum (by ref)"))
  ;[0.4039 0.3373 1] Add Card in Sequence
  (if (and (`self.ReadyToAdd`) (`self.SequenceIsOver`))
    (`KismetArrayLibrary.Array_Add` (`self.E_Action`) `New Card`)
    (set `self.Something in sequence` true)))

(event `Clear feed`
  ;[0.4039 0.3373 1] Clear action
  (`KismetArrayLibrary.Array_Clear` (`self.E_Action`))
  (set `self.Something in sequence` false)
  (set `self.IndexSequence` 0))

(event `Smallest Card`
  (bind _holesinsequence (`self.HolesInSequence`))
  ;[0.4039 0.3373 1] Find Smallest Removed Card
  (if (== (`KismetArrayLibrary.Array_Length` _holesinsequence) 1)
    (set `self.CurrentSmallest` (`|GetArrayItem` _holesinsequence))
    (set `self.ReadyToAdd` false)
    (else
      (set `self.CurrentSmallest` (`|GetArrayItem` _holesinsequence))
      (for _array_element _holesinsequence
        (if (< _array_element (`self.CurrentSmallest`))
          (set `self.CurrentSmallest` _array_element))))))

(event `GetRespawned`
  (bind _current_checkpoint (`self.Current Checkpoint`))
  ;[1 0.9333 0.1608] Respawn System
  (`self.Stop Timelines`)
  (`self.K2_TeleportTo` (+ (`self.K2_GetActorLocation` _current_checkpoint) (0.0 0.0 50.0)) (`self.K2_GetActorRotation` _current_checkpoint))
  (for _array_element (`/Game/Blueprint/EndOfSection/BP_Checkpoint.BP_Traps` (`self.Current Checkpoint`))
    (`/Game/Blueprint/Player/Effects/ProtoTraps/ProtoTrap.Reenable Trap` _array_element)))

(event `ChangeCheckpoint`
  (params (CurrentCheckpoint :type "/Game/Blueprint/EndOfSection/BP_Checkpoint Object Reference"))
  ;[1 0.9333 0.1608] Respawn System
  ;;[0.1059 0.05882 0.5137] Change Checkpoint
  (set `self.Current Checkpoint` CurrentCheckpoint))

(fn `UserConstructionScript`)