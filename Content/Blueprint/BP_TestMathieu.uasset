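; Test player Blueprint that executes a queued list of move-forward, turn-left and turn-right actions in order.
; PlaySequence delegates each action to BPMoveForward, which receives a player reference, as does the HUD_Movement widget created at BeginPlay.
; Move and rotation events lerp from the current transform with Timelines, each starting the next action on finish.
; Tick prints location and rotation for debugging.
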(event `PlaySequence`
  (bind _bp_moveforward (`self.BP_MoveForward`))
  (switch `/Game/Blueprint/E_ActionPlayer` (`|GetArrayItem` (`self.E_Action`) (`self.IndexSequence`))
    (:`NewEnumerator0`
      (`/Game/Blueprint/BP_MoveForward.MoveForward` _bp_moveforward))
    (:`NewEnumerator1`
      (`/Game/Blueprint/BP_MoveForward.TurnLeft` _bp_moveforward))
    (:`NewEnumerator2`
      (`/Game/Blueprint/BP_MoveForward.TurnRight` _bp_moveforward))))

(event `self.ReceiveBeginPlay`
  (bind _returnvalue (`|CreateWidget` "/Game/Blueprint/HUD_Movement.HUD_Movement_C" (`GameplayStatics.GetPlayerController` 0)))
  (`UserWidget.AddToViewport` _returnvalue 0)
  (set `/Game/Blueprint/HUD_Movement.PlayerRef` self _returnvalue)
  (set `/Game/Blueprint/BP_MoveForward.PlayerRef` self (`self.BP_MoveForward`)))

(event `MoveToDestination`
  (params (B :type "Vector Structure"))
  (bind (_direction _movetolocation) (`Timeline|MoveToDest` :!via `PlayFromStart`)
    (:`Update`
      (`self.K2_SetActorLocation` (`KismetMathLibrary.VLerp` (`self.K2_GetActorLocation`) B _movetolocation)))
    (:`Finished`
      (bind _result (`/Engine/EditorBlueprintResources/StandardMacros.IncrementInt` (`self.IndexSequence`))
        (:`  `
          (if (not (> _result (`KismetArrayLibrary.Array_LastIndex` (`self.E_Action`))))
            (`self.PlaySequence`)))))))

(event `self.ReceiveTick`
  (params (DeltaSeconds :type "Float (single-precision)"))
  (`KismetSystemLibrary.PrintString` (`KismetStringLibrary.Concat_StrStr` "Player Location : " (`KismetStringLibrary.Conv_VectorToString` (`self.K2_GetActorLocation`)) " | Player Rotation : " (`KismetStringLibrary.Conv_RotatorToString` (`self.K2_GetActorRotation`))) true true (struct :`G` 0.66 :`B` 1.0 :`A` 1.0) 0.0))

(event `RotationLeft`
  (params (B :type "Rotator Structure"))
  (bind (_direction _rotaleft) (`Timeline|RotaLeft` :!via `PlayFromStart`)
    (:`Update`
      (`self.K2_SetActorRotation` (`KismetMathLibrary.RLerp` (`self.K2_GetActorRotation`) B _rotaleft true)))
    (:`Finished`
      (bind _result (`/Engine/EditorBlueprintResources/StandardMacros.IncrementInt` (`self.IndexSequence`))
        (:`  `
          (if (not (> _result (`KismetArrayLibrary.Array_LastIndex` (`self.E_Action`))))
            (`self.PlaySequence`)))))))

(event `RotationRight`
  (params (B :type "Rotator Structure"))
  (bind (_direction _leftrota) (`Timeline|Timeline` :!via `PlayFromStart`)
    (:`Update`
      (`self.K2_SetActorRotation` (`KismetMathLibrary.RLerp` (`self.K2_GetActorRotation`) B _leftrota true)))
    (:`Finished`
      (bind _result (`/Engine/EditorBlueprintResources/StandardMacros.IncrementInt` (`self.IndexSequence`))
        (:`  `
          (if (not (> _result (`KismetArrayLibrary.Array_LastIndex` (`self.E_Action`))))
            (`self.PlaySequence`)))))))

(fn `UserConstructionScript`)