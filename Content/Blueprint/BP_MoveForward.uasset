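; BP_MoveForward is a movement command relay that turns step and turn events into target transforms for the player.
; Forward and diagonal up/down events offset the player's current location by a fixed step along its forward vector, the diagonals adding an equal vertical offset.
; Turn events offset yaw by a quarter turn.
; Each event passes its result to a matching PlayerRef function, which handles the movement or rotation.
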(event `DiagonalUp`
  (bind _playerref (`self.PlayerRef`))
  (`/Game/Blueprint/BP_MainCharacter.Diagonal Up` _playerref (+ (`Actor.K2_GetActorLocation` _playerref) (* (`Actor.GetActorForwardVector` _playerref) 100.0) (0.0 0.0 100.0))))

(event `MoveForward`
  (bind _playerref (`self.PlayerRef`))
  (`/Game/Blueprint/BP_MainCharacter.MoveToDestination` _playerref (+ (`Actor.K2_GetActorLocation` _playerref) (* (`Actor.GetActorForwardVector` _playerref) 100.0))))

(event `TurnLeft`
  (bind _playerref (`self.PlayerRef`))
  (`/Game/Blueprint/BP_MainCharacter.RotationLeft` _playerref (`KismetMathLibrary.MakeRotator` (.roll (`Actor.K2_GetActorRotation` _playerref)) (.pitch (`Actor.K2_GetActorRotation` _playerref)) (+ (.yaw (`Actor.K2_GetActorRotation` _playerref)) -90.0))))

(event `DiagonalDown`
  (bind _playerref (`self.PlayerRef`))
  (`/Game/Blueprint/BP_MainCharacter.DiagonalDown` _playerref (+ (`Actor.K2_GetActorLocation` _playerref) (* (`Actor.GetActorForwardVector` _playerref) 100.0) (0.0 0.0 -100.0))))

(event `TurnRight`
  (bind _playerref (`self.PlayerRef`))
  (`/Game/Blueprint/BP_MainCharacter.RotationRight` _playerref (`KismetMathLibrary.MakeRotator` (.roll (`Actor.K2_GetActorRotation` _playerref)) (.pitch (`Actor.K2_GetActorRotation` _playerref)) (+ (.yaw (`Actor.K2_GetActorRotation` _playerref)) 90.0))))